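; Game mode for a samurai quick-draw duel between the player and an NPC, driving the round through Intro, Wait, Draw and Finished phases.
; Tick times the intro, then a random delay opens the Draw phase, firing DrawPhaseStarted and revealing the exclamation cue.
; A successful attack defeats the opponent, hides the cue and starts a restart timer.
; Reset returns both samurai and the phase clock to Intro.
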(event `self.ReceiveBeginPlay`
  (bind _returnvalue (`GameplayStatics.GetActorOfClass` "/Game/Blueprints/BP_Exclamation.BP_Exclamation_C"))
  (set `self.ExclamationRef` _returnvalue)
  (bind _returnvalue_2 (`GameplayStatics.GetActorOfClass` "/Game/Blueprints/BP_Samurai_Player.BP_Samurai_Player_C"))
  (set `self.SamuraiPlayer` _returnvalue_2)
  (bind _returnvalue_3 (`GameplayStatics.GetActorOfClass` "/Game/Blueprints/BP_Samurai_NPC.BP_Samurai_NPC_C"))
  (set `self.SamuraiNpc` _returnvalue_3))

(event `self.ReceiveTick`
  (params (DeltaSeconds :type "Float (single-precision)"))
  (set `self.ElaspedTime` (+ DeltaSeconds (`self.ElaspedTime`)))
  (switch `/Game/Blueprints/Enums/E_Phase` (`self.Phase`)
    (:`NewEnumerator0`
      (if (>= (`self.ElaspedTime`) (`self.RoundStartTime`))
        (set `self.Phase` "NewEnumerator1")
        (`KismetSystemLibrary.Delay` (`KismetMathLibrary.RandomFloatInRange` (`self.MinDrawDelay`) (`self.MaxDrawDelay`)))
        (set `self.Phase` "NewEnumerator2")
        (`self.DrawPhaseStarted`)
        (`/Engine/EditorBlueprintResources/StandardMacros.IsValid` (`self.ExclamationRef`)
          (:`Is Valid`
            (`/Game/Blueprints/BP_Exclamation.SetVisibility` (`self.ExclamationRef`) true))
          (:`Is Not Valid`
            (`KismetSystemLibrary.PrintString` "Exclamation Not Found")))))))

(fn `AttackedSuccessfully`
  (params (IsPlayer :type Boolean))
  (if IsPlayer
    (`/Game/Blueprints/BP_Samurai.Defeated` (`self.SamuraiNpc`))
    (else
      (`/Game/Blueprints/BP_Samurai.Defeated` (`self.SamuraiPlayer`))))
  (`/Engine/EditorBlueprintResources/StandardMacros.IsValid` (`self.ExclamationRef`)
    (:`Is Valid`
      (`/Game/Blueprints/BP_Exclamation.SetVisibility` (`self.ExclamationRef`) false)
      (`KismetSystemLibrary.K2_SetTimerDelegate` (`|CreateDelegate` :!event `Reset`) (`self.RestartDelay`)))))

(fn `Reset`
  (set `self.Phase` "NewEnumerator0")
  (set `self.ElaspedTime` 0.0)
  (`/Game/Blueprints/BP_Samurai.Reset` (`self.SamuraiPlayer`))
  (`/Game/Blueprints/BP_Samurai.Reset` (`self.SamuraiNpc`)))

(fn `SetGameFinished`
  (set `self.Phase` "NewEnumerator3"))

(fn `UserConstructionScript`)